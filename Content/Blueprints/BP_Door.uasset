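; Door Blueprint that raises and lowers a Door component when its DoorOpen event fires, provided DoorScore equals the required value.
; DoorOpen plays or reverses the DoorAnimation timeline based on the Open flag, lerping the relative location between DoorStart and DoorEnd.
; Open flips when the timeline finishes; a separate OpenDoor function also toggles the flag but is not called here.
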(event `DoorOpen`
  (if (== (`self.DoorScore`) 5)
    (if (`self.Open`)
      (bind (_direction _doorraise) (`Timeline|DoorAnimation` :!via `Reverse` :!label _label)
        (:`Update`
          (`SceneComponent.K2_SetRelativeLocation` (`self.Door`) (`KismetMathLibrary.VLerp` (`self.DoorStart`) (`self.DoorEnd`) _doorraise) false false))
        (:`Finished`
          (set `self.Open` (not (`self.Open`)))))
      (else
        (goto _label)))))

(fn `OpenDoor`
  (set `self.Open` (not (`self.Open`))))

(fn `UserConstructionScript`)