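; Spikes is a moving hazard actor that fails the level when overlapped.
; On BeginPlay it stores its starting location and plays the Moving timeline, which offsets the actor from that point without sweeping.
; Any actor overlap, with no check on the other actor, shows the mouse cursor and adds a LevelFail widget to the viewport.
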(event `self.ReceiveBeginPlay`
  ;[1 1 1] Movement of Spike
  (set `self.Starting Location` (`self.K2_GetActorLocation`))
  (bind (_direction _movement) (`Timeline|Moving` :!via `PlayFromStart`)
    (:`Update`
      (`self.K2_SetActorLocation` (+ (`self.Starting Location`) _movement)))))

(event `self.ReceiveActorBeginOverlap`
  (params (OtherActor :type "Actor Object Reference"))
  ;[1 1 1] Die When Hit
  (bind _returnvalue (`|CreateWidget` "/Game/Widgets/LevelFail.LevelFail_C"))
  (set `PlayerController.bShowMouseCursor` true (`GameplayStatics.GetPlayerController` 0))
  (`UserWidget.AddToViewport` _returnvalue 0))

(fn `UserConstructionScript`)