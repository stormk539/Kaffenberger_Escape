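; BP_Button is a button actor that slides a referenced BP_Door open when its Button component is hit.
; The hit event checks that player pawn 0 is a FirstPersonCharacter, not what hit it, then plays a timeline.
; The timeline lerps the door root's relative location from DoorStart to DoorEnd.
; On finish it flips Open, which this graph never reads, and nothing reverses the motion.
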(event `self.Button.OnComponentHit`
  (params (HitComponent :type "PrimitiveComponent Object Reference") (OtherActor :type "Actor Object Reference") (OtherComp :type "PrimitiveComponent Object Reference") (NormalImpulse :type "Vector Structure") (Hit :type "HitResult Structure (by ref)"))
  ;[1 1 1] Target Button
  (cast `/Game/FirstPersonBP/Blueprints/FirstPersonCharacter` (`GameplayStatics.GetPlayerPawn` 0))
  (cast `/Game/Blueprints/BP_Door` (`self.Door`))
  (bind (_direction _door_opening) (`Timeline|Timeline_0`)
    (:`Update`
      (`SceneComponent.K2_SetRelativeLocation` (`Actor.RootComponent` (`self.Door`)) (`KismetMathLibrary.VLerp` (`self.Door Start`) (`self.Door End`) _door_opening) false false))
    (:`Finished`
      (set `self.Open` (not (`self.Open`))))))

(fn `UserConstructionScript`)